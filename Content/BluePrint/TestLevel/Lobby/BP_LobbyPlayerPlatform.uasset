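; Lobby platform Blueprint that displays a BP_Player character for an assigned player controller (PC).
; SpawnCharacter stores the PC, destroys any existing character, then spawns and tracks a new BP_Player at the platform's spawn transform component.
; Clear releases the PC reference and destroys the displayed character.
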(event Custom|SpawnCharacter
  (params (PC :type Player%20Controller%20Object%20Reference))
  (Variables|Default|SetPC PC)
  (Utilities|IsValid (Variables|Default|GetCurrentCharcter)
    (:Is%20Valid
      (Actor|DestroyActor (Variables|Default|GetCurrentCharcter)))
    (:Is%20Not%20Valid
      _))
  (bind _returnvalue (Game|SpawnActorfromClass "/Game/BluePrint/TestLevel/TestPlay/BP_Player.BP_Player_C" (Transformation|GetWorldTransform (Variables|Default|GetplayerSpawnTrasnform)) "Undefined" "MultiplyWithRoot" 0 0))
  (Variables|Default|SetCurrentCharcter _returnvalue))

(event Custom|Clear
  (Variables|Default|SetPC 0)
  (Utilities|IsValid (Variables|Default|GetCurrentCharcter)
    (:Is%20Valid
      (Actor|DestroyActor (Variables|Default|GetCurrentCharcter))
      (Variables|Default|SetCurrentCharcter 0))))

(fn ConstructionScript)