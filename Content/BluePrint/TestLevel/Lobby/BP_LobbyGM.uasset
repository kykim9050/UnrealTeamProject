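; Lobby game mode that assigns each joined player controller to a player platform, where a character is spawned for it.
; On BeginPlay it builds an ordered platform list by matching actor tags to index numbers.
; Login and logout update the controller list, wait through a short-delay polling macro until setup finishes, then reconcile platforms.
; Reconciliation fills the first free platform for each unplaced player and clears platforms whose controller is no longer listed.
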(event EventBeginPlay
  (CallFunction|SetUpPlatforms))

(event EventPostLogin
  (params (NewPlayer :type Player%20Controller%20Object%20Reference))
  (Utilities|Array|Add (Variables|Default|GetPCs) NewPlayer)
  (Utilities|IfPlatformSetUpIsDone
    (:True
      (CallFunction|UpdatePlayersonPlatforms))))

(event EventOnLogout
  (params (ExitingController :type Controller%20Object%20Reference))
  (bind _as플레이어_컨트롤러 (Utilities|Casting|CastToPlayerController ExitingController))
  (Utilities|Array|RemoveItem (Variables|Default|GetPCs) _as플레이어_컨트롤러)
  (Utilities|IfPlatformSetUpIsDone
    (:True
      (CallFunction|UpdatePlayersonPlatforms))))

(fn ConstructionScript)

(fn SetUpPlatforms
  (bind _outactors (Actor|GetAllActorsOfClass "/Game/BluePrint/TestLevel/Lobby/BP_LobbyPlayerPlatform.BP_LobbyPlayerPlatform_C"))
  (for _index (range 0 (Utilities|Array|LastIndex _outactors))
    (bind _outactors_2 (Actor|GetAllActorsOfClasswithTag "/Game/BluePrint/TestLevel/Lobby/BP_LobbyPlayerPlatform.BP_LobbyPlayerPlatform_C" (Utilities|String|StringToName (Utilities|String|ToString(Integer) _index))))
    (Utilities|Array|Add (Variables|Default|GetPlayerPlatforms) (Utilities|Array|Get(acopy) _outactors_2)))
  (Variables|Default|SetbPlatformSetUoDone true))

(fn UpdatePlayersonPlatforms
  ;[1 1 1] 코멘트
  (for _array_element (Variables|Default|GetPCs)
    (LocalVariables|SetLoop_PcAlreadyAdded false)
    (bind _array_element_2 (Utilities|Array|ForEachLoopwithBreak (Variables|Default|GetPlayerPlatforms) :!label _label)
      (:LoopBody
        (if (== (Variables|/Game/BluePrint/TestLevel/Lobby/BP_LobbyPlayerPlatform.BP_LobbyPlayerPlatform_C|GetPC _array_element_2) _array_element)
          (LocalVariables|SetLoop_PcAlreadyAdded true)
          (goto _label Break)))
      (:Completed
        ;[1 1 1] 코멘트
        (if (not (LocalVariables|GetLoop_PcAlreadyAdded))
          (bind _array_element_3 (Utilities|Array|ForEachLoopwithBreak (Variables|Default|GetPlayerPlatforms) :!label _label_2)
            (:LoopBody
              (Utilities|IsValid (Variables|/Game/BluePrint/TestLevel/Lobby/BP_LobbyPlayerPlatform.BP_LobbyPlayerPlatform_C|GetPC _array_element_3)
                (:Is%20Not%20Valid
                  (Default|SpawnCharacter _array_element_3 _array_element)
                  (goto _label_2 Break)))))))))
  ;[1 1 1] 코멘트
  (for _array_element_4 (Variables|Default|GetPlayerPlatforms)
    (if (not (Utilities|Array|ContainsItem (Variables|Default|GetPCs) (Variables|/Game/BluePrint/TestLevel/Lobby/BP_LobbyPlayerPlatform.BP_LobbyPlayerPlatform_C|GetPC _array_element_4)))
      (Default|Clear _array_element_4))))