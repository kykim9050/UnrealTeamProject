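; Test-level player controller that adds the IC_Player Enhanced Input mapping context and sets game-only input on BeginPlay.
; Four directional actions move the controlled pawn along its own forward and right vectors, negated for back and left.
; Mouse rotation drives yaw and inverted-Y pitch, each scaled by the action's elapsed seconds.
; Jump acts on player character 0 rather than the controlled pawn.
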(event Input|EnhancedActionEvents|EnhancedInputActionIA_LeftMove
  (params (ActionValue :type Boolean) (ElapsedSeconds :type Float%20%28double-precision%29) (TriggeredSeconds :type Float%20%28double-precision%29) (InputAction :type Input%20Action%20Object%20Reference :default "/Game/Resources/TestLevel/Input/IA_LeftMove.IA_LeftMove"))
  (bind _returnvalue (Pawn|GetControlledPawn))
  (Pawn|Input|AddMovementInput _returnvalue (Math|Vector|NegateVector (Math|Vector|GetRightVector (.Rotation (Math|Transform|BreakTransform (Transformation|GetActorTransform _returnvalue))))) 1.0 false))

(event Input|EnhancedActionEvents|EnhancedInputActionIA_Jump
  (params (ActionValue :type Boolean) (ElapsedSeconds :type Float%20%28double-precision%29) (TriggeredSeconds :type Float%20%28double-precision%29) (InputAction :type Input%20Action%20Object%20Reference :default "/Game/Resources/TestLevel/Input/IA_Jump.IA_Jump"))
  (Character|Jump (Game|GetPlayerCharacter 0)))

(event Input|EnhancedActionEvents|EnhancedInputActionIA_MouseRotation
  (params (ActionValue :type Vector%202D%20Structure) (ElapsedSeconds :type Float%20%28double-precision%29) (TriggeredSeconds :type Float%20%28double-precision%29) (InputAction :type Input%20Action%20Object%20Reference :default "/Game/Resources/TestLevel/Input/IA_MouseRotation.IA_MouseRotation"))
  ;[1 1 1] 코멘트
  (Class|PlayerController|AddPitchInput (* (.Y (Math|Vector2D|BreakVector2D (Class|KismetMathLibrary|Negated2D ActionValue))) ElapsedSeconds)))

(event Input|EnhancedActionEvents|EnhancedInputActionIA_MouseRotation
  (params (ActionValue :type Vector%202D%20Structure) (ElapsedSeconds :type Float%20%28double-precision%29) (TriggeredSeconds :type Float%20%28double-precision%29) (InputAction :type Input%20Action%20Object%20Reference :default "/Game/Resources/TestLevel/Input/IA_MouseRotation.IA_MouseRotation"))
  (Class|PlayerController|AddYawInput (* (.X (Math|Vector2D|BreakVector2D ActionValue)) ElapsedSeconds)))

(event Input|EnhancedActionEvents|EnhancedInputActionIA_FrontMove
  (params (ActionValue :type Boolean) (ElapsedSeconds :type Float%20%28double-precision%29) (TriggeredSeconds :type Float%20%28double-precision%29) (InputAction :type Input%20Action%20Object%20Reference :default "/Game/Resources/TestLevel/Input/IA_FrontMove.IA_FrontMove"))
  (bind _returnvalue (Pawn|GetControlledPawn))
  (Pawn|Input|AddMovementInput _returnvalue (Math|Vector|GetForwardVector (.Rotation (Math|Transform|BreakTransform (Transformation|GetActorTransform _returnvalue)))) 1.0 false))

(event Input|EnhancedActionEvents|EnhancedInputActionIA_BackMove
  (params (ActionValue :type Boolean) (ElapsedSeconds :type Float%20%28double-precision%29) (TriggeredSeconds :type Float%20%28double-precision%29) (InputAction :type Input%20Action%20Object%20Reference :default "/Game/Resources/TestLevel/Input/IA_BackMove.IA_BackMove"))
  (bind _returnvalue (Pawn|GetControlledPawn))
  (Pawn|Input|AddMovementInput _returnvalue (Math|Vector|NegateVector (Math|Vector|GetForwardVector (.Rotation (Math|Transform|BreakTransform (Transformation|GetActorTransform _returnvalue))))) 1.0 false))

(event Input|EnhancedActionEvents|EnhancedInputActionIA_RightMove
  (params (ActionValue :type Boolean) (ElapsedSeconds :type Float%20%28double-precision%29) (TriggeredSeconds :type Float%20%28double-precision%29) (InputAction :type Input%20Action%20Object%20Reference :default "/Game/Resources/TestLevel/Input/IA_RightMove.IA_RightMove"))
  (bind _returnvalue (Pawn|GetControlledPawn))
  (Pawn|Input|AddMovementInput _returnvalue (Math|Vector|GetRightVector (.Rotation (Math|Transform|BreakTransform (Transformation|GetActorTransform _returnvalue)))) 1.0 false))

(event EventBeginPlay
  (Input|AddMappingContext (PlayerController|LocalPlayerSubsystems|GetEnhancedInputLocalPlayerSubsystem self) "/Game/Resources/TestLevel/Input/IC_Player.IC_Player" 0 "(bIgnoreAllPressedKeysUntilRelease=True,bForceImmediately=False,bNotifyUserSettings=False)")
  (Input|SetInputModeGameOnly self false))

(event EventTick
  (params (DeltaSeconds :type Float%20%28single-precision%29)))

(fn ConstructionScript)