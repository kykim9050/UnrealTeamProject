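; BP_TestSample is a test object actor that shows an E-key widget while the player is within its collision.
; On BeginPlay it calls SetInfo with "Sample" and creates the E_Key widget once, keeping a reference.
; CollisionComponent overlap events add that widget to the viewport when the player pawn enters and remove it when the pawn leaves.
; It handles no key input itself.
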(event OnComponentBeginOverlap(CollisionComponent)
  (params (OverlappedComponent :type Primitive%20Component%20Object%20Reference) (OtherActor :type Actor%20Object%20Reference) (OtherComp :type Primitive%20Component%20Object%20Reference) (OtherBodyIndex :type Integer) (bFromSweep :type Boolean) (SweepResult :type Hit%20Result%20Structure%20%28by%20ref%29))
  (if (== OtherActor (Game|Player|GetPlayerPawn 0))
    (UserInterface|Viewport|AddtoViewport (Variables|Default|GetE_KEY) 0)))

(event OnComponentEndOverlap(CollisionComponent)
  (params (OverlappedComponent :type Primitive%20Component%20Object%20Reference) (OtherActor :type Actor%20Object%20Reference) (OtherComp :type Primitive%20Component%20Object%20Reference) (OtherBodyIndex :type Integer))
  (if (== OtherActor (Game|Player|GetPlayerPawn 0))
    (Widget|RemovefromParent (Variables|Default|GetE_KEY))))

(event EventBeginPlay
  (Class|MapObjectBase|SetInfo "Sample")
  (bind _returnvalue (UserInterface|CreateWidget "/Game/BluePrint/PartDevLevel/UI/Interact_E/E_Key.E_Key_C"))
  (Variables|Default|SetE_KEY _returnvalue))

(event Collision|EventActorBeginOverlap
  (params (OtherActor :type Actor%20Object%20Reference)))

(event EventTick
  (params (DeltaSeconds :type Float%20%28single-precision%29)))

(fn ConstructionScript)