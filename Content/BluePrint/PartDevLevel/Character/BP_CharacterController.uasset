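; Player controller that gives the local player a chat panel and relays chat messages to every player.
; BeginPlay creates the chat widget, and Enter moves keyboard focus to its input box.
; SR_SubmiChat loops the GameState's PlayerArray, calling each controller's OC update event to refresh its panel.
; Tick also runs a test raycast on player 0's TestCharacter with zeroed position and rotation.
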(event Custom|SR_SubmiChat
  (params (PlayerName :type Text) (ChatMassage :type Text))
  ;[1 1 1] 채팅창(UI)
  (for _array_element (Variables|/Script/Engine.GameStateBase|GetPlayerArray (Game|GetGameState))
    (bind _asbp_character_controller (Utilities|Casting|CastToBP_CharacterController (Game|GetPlayerController _array_element)))
    (CallFunction|OCUpdateChat _asbp_character_controller PlayerName ChatMassage)))

(event Custom|OC_UpdateChat
  (params (Player%20Name :type Text) (Chat%20Massage :type Text))
  ;[1 1 1] 채팅창(UI)
  (bind _wb_chat_panel_ (Variables|Default|GetWB_Chat%20Panel%20)
    (:then
      (Default|UpdateChat _wb_chat_panel_ Player%20Name Chat%20Massage))
    (:else)))

(event Input|EnhancedActionEvents|EnhancedInputActionIA_MouseRight
  (params (ActionValue :type Boolean) (ElapsedSeconds :type Float%20%28double-precision%29) (TriggeredSeconds :type Float%20%28double-precision%29) (InputAction :type Input%20Action%20Object%20Reference :default "/Game/Resources/TestLevel/Input/IA_MouseRight.IA_MouseRight"))
  ;[1 1 1] Character 에 있는 RayCast 실행.(TEST)
)

(event EventBeginPlay
  ;[1 1 1] 플레이어에게 채팅창 좌측하단에 생성(UI)
  (if (Pawn|IsLocalController)
    (bind _returnvalue (UserInterface|CreateWidget "/Game/BluePrint/PartDevLevel/UI/chat/WB_ChatPanel.WB_ChatPanel_C" self))
    (bind _output_get (Variables|Default|SetWB_Chat%20Panel%20 _returnvalue))
    (UserInterface|Viewport|AddtoViewport _output_get 0)))

(event EventTick
  (params (DeltaSeconds :type Float%20%28single-precision%29))
  ;[1 1 1] Character 에 있는 RayCast 실행.(TEST)
  (bind _astest_character (Utilities|Casting|CastToTestCharacter (Game|Player|GetPlayerPawn 0)))
  (Class|TestCharacter|CreateRayCast _astest_character 0.0 (Math|Vector|MakeVector 0.0 0.0 0.0) "0, 0, 0" (Math|Rotator|MakeRotator 0.0 0.0 0.0)))

(event Input|KeyboardEvents|Enter
  (params (Key :type Key%20Structure :default "None"))
  ;[1 1 1] 채팅창(UI)
  ;;[1 1 1] 엔터시 채팅창으로 키보드 포커스 이동
  (:Pressed
    (bind _wb_chat_panel_ (Variables|Default|GetWB_Chat%20Panel%20)
      (:then
        (Widget|SetKeyboardFocus (Variables|/Game/BluePrint/PartDevLevel/UI/chat/WB_ChatPanel.WB_ChatPanel_C|GetChatInputBox _wb_chat_panel_)))
      (:else))))

(fn ConstructionScript)