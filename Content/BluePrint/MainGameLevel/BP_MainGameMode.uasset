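; Game mode for the main game level that keeps a list of connected players and shares it with their controllers.
; PostLogin and OnLogout add or remove player controllers in AllPCs, then call Updatelist.
; Updatelist rebuilds the list from PlayerState names with every score set to zero, then passes it to each BP_GmaplayerPC through UpdateplayerListPC.
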(event EventBeginPlay)

(event EventTick
  (params (DeltaSeconds :type Float%20%28single-precision%29)))

(event EventPostLogin
  (params (NewPlayer :type Player%20Controller%20Object%20Reference))
  (Utilities|Array|Add (Variables|Default|GetAllPCs) NewPlayer)
  (CallFunction|Updatelist))

(event EventOnLogout
  (params (ExitingController :type Controller%20Object%20Reference))
  (bind _as플레이어_컨트롤러 (Utilities|Casting|CastToPlayerController ExitingController))
  (Utilities|Array|RemoveItem (Variables|Default|GetAllPCs) _as플레이어_컨트롤러)
  (CallFunction|Updatelist))

(fn ConstructionScript)

(fn Updatelist
  (Utilities|Array|Clear (Variables|Default|Getlist))
  (for _array_element (Variables|Default|GetAllPCs)
    (Utilities|Array|Add (Variables|Default|Getlist) (Utilities|Struct|MakeBP_struc (Utilities|Text|ToText(String) (PlayerState|GetPlayerName (Variables|/Script/Engine.Controller|GetPlayerState _array_element))))))
  (for _array_element_2 (Variables|Default|GetAllPCs)
    (bind _asbp_gmaplayer_pc (Utilities|Casting|CastToBP_GmaplayerPC _array_element_2))
    (Default|UpdateplayerListPC _asbp_gmaplayer_pc (Variables|Default|Getlist))))